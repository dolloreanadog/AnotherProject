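; BP_PUHealth is a health pickup that heals the player who overlaps it.
; When its Collider begins overlapping an actor, it gets the player through a GetPlayer call on that actor and calls Heal with a fixed amount.
; It then prints the returned health value as a debug string and destroys itself.
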(event OnComponentBeginOverlap(Collider)
  (params (OverlappedComponent :type Primitive%20Component%20Object%20Reference) (OtherActor :type Actor%20Object%20Reference) (OtherComp :type Primitive%20Component%20Object%20Reference) (OtherBodyIndex :type Integer) (bFromSweep :type Boolean) (SweepResult :type Hit%20Result%20Structure%20%28by%20ref%29))
  (bind _asbp_wagon_character (CallFunction|GetPlayer OtherActor OtherActor))
  (bind _returnvalue (Class|WagonCharacter|Heal _asbp_wagon_character 1e+02))
  (Development|PrintString (Utilities|String|Append "Player Health: " (Utilities|String|ToString(Float) _returnvalue)))
  (Actor|DestroyActor))

(event EventBeginPlay
  (|CallParentFunction) ; This node is disabled and will not be called.\nDrag off pins to build functionality.
)

(event Collision|EventActorBeginOverlap
  (params (OtherActor :type Actor%20Object%20Reference)))

(event EventTick
  (params (DeltaSeconds :type Float%20%28single-precision%29))
  (|CallParentFunction DeltaSeconds) ; This node is disabled and will not be called.\nDrag off pins to build functionality.
)

(fn ConstructionScript
  (|CallParentFunction))