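; BP_PUStun is a pickup that resets the player's stun on overlap.
; When its Collider begins overlapping an actor, it gets the player from that actor, calls ResetStun and passes CurrentStunCount to the player UI.
; It then plays the Ammo sound at its location, prints a debug "Hello" and destroys itself.
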(event OnComponentBeginOverlap(Collider)
  (params (OverlappedComponent :type Primitive%20Component%20Object%20Reference) (OtherActor :type Actor%20Object%20Reference) (OtherComp :type Primitive%20Component%20Object%20Reference) (OtherBodyIndex :type Integer) (bFromSweep :type Boolean) (SweepResult :type Hit%20Result%20Structure%20%28by%20ref%29))
  (bind _asbp_wagon_character (CallFunction|GetPlayer OtherActor OtherActor))
  (Class|WagonCharacter|ResetStun _asbp_wagon_character)
  (Default|GetStuns (Variables|/Game/Character/BP_Wagon_Character.BP_Wagon_Character_C|GetPlayerUI _asbp_wagon_character) (Variables|/Script/AnotherProject.Wagon_Character|Get_currentStunCount _asbp_wagon_character))
  (Audio|SpawnSoundatLocation "/Game/Audio/SFX/Ammo.Ammo" (Transformation|GetActorLocation) "0, 0, 0" 1.0 1.0 0.0 0 0)
  (Development|PrintString "Hello")
  (Actor|DestroyActor))

(event EventBeginPlay
  (|CallParentFunction) ; This node is disabled and will not be called.\nDrag off pins to build functionality.
)

(event Collision|EventActorBeginOverlap
  (params (OtherActor :type Actor%20Object%20Reference)))

(event EventTick
  (params (DeltaSeconds :type Float%20%28single-precision%29))
  (|CallParentFunction DeltaSeconds) ; This node is disabled and will not be called.\nDrag off pins to build functionality.
)

(fn ConstructionScript
  (|CallParentFunction))