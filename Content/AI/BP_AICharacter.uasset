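; AI enemy character that punches the player on contact and reacts to stun and death events.
; A HurtTrigger overlap damages Player-tagged actors, then disables movement and further attacks for a short delay before restoring NavWalking.
; Punch, dizzy and death animations play directly on the mesh, overriding the Animation Blueprint, which is restored on stun end.
; Tick copies IsStunned into the AI controller's Blackboard every frame.
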(event OnComponentBeginOverlap(HurtTrigger)
  (params (OverlappedComponent :type Primitive%20Component%20Object%20Reference) (OtherActor :type Actor%20Object%20Reference) (OtherComp :type Primitive%20Component%20Object%20Reference) (OtherBodyIndex :type Integer) (bFromSweep :type Boolean) (SweepResult :type Hit%20Result%20Structure%20%28by%20ref%29))
  (bind _charactermovement (Variables|Character|GetCharacterMovement))
  (if (Variables|Default|GetCanAttack)
    (if (Actor|ActorHasTag OtherActor "Player")
      (Variables|Default|SetCanAttack false)
      (Game|Damage|ApplyDamage OtherActor 5e+01 0 self)
      (Components|Animation|PlayAnimation (Variables|Character|GetMesh) "/Game/ControlRig/Characters/Mannequins/Animations/Quinn/Punching_Anim.Punching_Anim" false)
      (Pawn|Components|CharacterMovement|DisableMovement _charactermovement)
      (Utilities|FlowControl|Delay 3.0)
      (Variables|Default|SetCanAttack true)
      (Pawn|Components|CharacterMovement|SetMovementMode _charactermovement "MOVE_NavWalking" 0))))

(event Custom|On%20Stun
  (params (Duration :type Float%20%28single-precision%29))
  (Components|Animation|PlayAnimation (Variables|Character|GetMesh) "/Game/ControlRig/Characters/Mannequins/Animations/Quinn/Dizzy_Idle_Anim.Dizzy_Idle_Anim" false))

(event Custom|On%20Stun%20End
  (Components|Animation|SetAnimationMode (Variables|Character|GetMesh) "AnimationBlueprint" true))

(event Custom|On%20Death
  (Components|Animation|PlayAnimation (Variables|Character|GetMesh) "/Game/ControlRig/Characters/Mannequins/Animations/Manny/Death_From_Right_Anim.Death_From_Right_Anim" false))

(event EventBeginPlay
  (EventDispatchers|BindEventtoOnDeath (delegate Custom|On%20Death))
  (EventDispatchers|BindEventtoOnStun (delegate Custom|On%20Stun))
  (EventDispatchers|BindEventtoOnStunEnd (delegate Custom|On%20Stun%20End)))

(event Collision|EventActorBeginOverlap
  (params (OtherActor :type Actor%20Object%20Reference)))

(event EventTick
  (params (DeltaSeconds :type Float%20%28single-precision%29))
  (bind _asaicontroller (Utilities|Casting|CastToAIController (Pawn|GetController))
    (:then
      (AI|Components|Blackboard|SetValueasBool (AI|GetBlackboard _asaicontroller) (Variables|Default|GetIsStunned) (Variables|Default|Get_isStunned)))
    (:CastFailed
      (Development|PrintString "Cast Has Failed!"))))

(fn ConstructionScript)