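; Player character that carries a limited-use area stun and manages its own HUD and menus.
; Q checks StunUsed, then stuns every BP_AICharacter in a large sphere overlap, spawning explosions at the player and refreshing stun count and cooldown on PlayerUI.
; Tick pushes health to the HUD, bound death and stun events play animations, and a debug key applies self-damage.
; ChangeMenuUI swaps menu widgets by index, toggling pause and cursor.
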(event Custom|On%20Death
  (Components|Animation|PlayAnimation (Variables|Character|GetMesh) "/Game/ControlRig/Characters/Mannequins/Animations/Manny/Death_From_Right_Anim.Death_From_Right_Anim" false))

(event Custom|On%20Stun
  (params (Duration :type Float%20%28single-precision%29))
  (Components|Animation|PlayAnimation (Variables|Character|GetMesh) "/Game/ControlRig/Characters/Mannequins/Animations/Quinn/Dizzy_Idle_Anim.Dizzy_Idle_Anim" false))

(event EventBeginPlay
  (EventDispatchers|BindEventtoOnDeath (delegate Custom|On%20Death))
  (EventDispatchers|BindEventtoOnStun (delegate Custom|On%20Stun))
  (Development|PrintString (Utilities|String|Append "Stun Uses: " (Utilities|String|ToString(Integer) (Variables|Default|Get_currentStunCount))))
  (bind _returnvalue (UserInterface|CreateWidget "/Game/UI/PlayerUI.PlayerUI_C"))
  (Variables|Default|SetPlayerUI _returnvalue)
  (UserInterface|Viewport|AddtoViewport _returnvalue 0)
  (Default|GetStuns (Variables|Default|GetPlayerUI) (Variables|Default|GetmaxStunCount)))

(event Collision|EventActorBeginOverlap
  (params (OtherActor :type Actor%20Object%20Reference)))

(event EventTick
  (params (DeltaSeconds :type Float%20%28single-precision%29))
  (Default|GetHealth (Variables|Default|GetPlayerUI) (Variables|Default|Get_currentHealth)))

(event Input|KeyboardEvents|DebugKey0
  (params (Key :type Key%20Structure :default "None") (ActionValue :type Input%20Action%20Value%20Structure))
  (:Pressed
    (Game|Damage|ApplyDamage self 1e+02 0 0)))

(event Input|KeyboardEvents|Q
  (params (Key :type Key%20Structure :default "None"))
  (bind _playerui (Variables|Default|GetPlayerUI))
  (:Pressed
    (bind _returnvalue (Class|WagonCharacter|StunUsed))
    (if _returnvalue
      (bind _outactors (Collision|SphereOverlapActors (Transformation|GetActorLocation) 1e+04 (Variables|Default|GetObject%20Types) "/Game/AI/BP_AICharacter.BP_AICharacter_C"))
      (for _array_element _outactors
        (bind _asbp_aicharacter (Utilities|Casting|CastToBP_AICharacter _array_element)
          (:then
            (Class|WagonCharacter|Stun _asbp_aicharacter 5.0)
            (Effects|SpawnEmitteratLocation "/Game/StarterContent/Particles/P_Explosion.P_Explosion" (Transformation|GetActorLocation self) "0, 0, 0" "3.000000,3.000000,3.000000")
            (Default|GetStuns _playerui (Variables|Default|Get_currentStunCount))
            (Default|GetStunCooldown _playerui (Variables|Default|Get_stunUseCooldown))
            (Development|PrintString "Done with stunning")
            (Development|PrintString (Utilities|String|Append "Done with stunning: " (Utilities|GetDisplayName _array_element))))
          (:CastFailed
            (Development|PrintString "Failed to stun"))))
      (else
        (Development|PrintString (Utilities|String|Append (Utilities|String|Append (Utilities|String|Append "Cannot Stun, " (Utilities|String|ToString(Float) (Variables|Default|Get_stunUseCooldown))) ", ") (Utilities|String|ToString(Integer) (Variables|Default|Get_currentStunCount))))))))

(fn ConstructionScript)

(fn ChangeMenuUI
  (params (uiValue :type Integer))
  (if (Utilities|IsValid (Variables|Default|GetMenuUI))
    (Widget|RemovefromParent (Variables|Default|GetMenuUI)))
  (switch int uiValue
    (:Default
      ;[0.15 0.15 0.15 0.5] Remove Menus
      (Utilities|String|LogString "Not Valid Menu" :!label _label)
      (Game|SetGamePaused false)
      (Variables|/Script/Engine.PlayerController|SetbShowMouseCursor (Game|GetPlayerController 0) false)
      (Game|SetGamePaused false))
    (:0
      (goto _label))
    (:1
      ;[0.15 0.15 0.15 0.5] Main Menu
      (bind _returnvalue (UserInterface|CreateWidget "/Game/UI/MainMenu.MainMenu_C"))
      (Variables|Default|SetMenuUI _returnvalue)
      (UserInterface|Viewport|AddtoViewport _returnvalue 0)
      (Variables|/Script/Engine.PlayerController|SetbShowMouseCursor (Game|GetPlayerController 0) true :!label _label_2)
      (Game|SetGamePaused true))
    (:2
      ;[0.15 0.15 0.15 0.5] Pause Menu
      (bind _returnvalue_2 (UserInterface|CreateWidget "/Game/UI/PauseMenu.PauseMenu_C"))
      (Variables|Default|SetMenuUI _returnvalue_2)
      (UserInterface|Viewport|AddtoViewport _returnvalue_2 0)
      (Game|SetGamePaused true :!label _label_3)
      (goto _label_2))
    (:3
      ;[0.15 0.15 0.15 0.5] Victory Menu
      (bind _returnvalue_3 (UserInterface|CreateWidget "/Game/UI/OverMenu.OverMenu_C"))
      (Variables|Default|SetMenuUI _returnvalue_3)
      (UserInterface|Viewport|AddtoViewport _returnvalue_3 0)
      (goto _label_3))
    (:4
      ;[0.15 0.15 0.15 0.5] Over Menu
      (bind _returnvalue_4 (UserInterface|CreateWidget "/Game/UI/VictoryMenu.VictoryMenu_C"))
      (Variables|Default|SetMenuUI _returnvalue_4)
      (UserInterface|Viewport|AddtoViewport _returnvalue_4 0)
      (goto _label_3))))

(fn ShowPlayerUI
  (params (Visible :type Boolean))
  (bind _playerui (Variables|Default|GetPlayerUI))
  (if Visible
    (Variables|/Script/UMG.Widget|SetVisibility _playerui "Visible")
    (else
      (Variables|/Script/UMG.Widget|SetVisibility _playerui "Hidden"))))